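; BP_Ball_01 is a player-controlled rolling ball that fades the screen in from opaque when play begins.
; Forward/back and left/right input axes apply scaled torque to the ball as an acceleration change, so movement comes from physics.
; Any damage triggers a one-time dark red camera fade starting from opaque, then reopens Level01 after a short delay, before the fade finishes.
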(event Game|Damage|EventAnyDamage
  (params (Damage :type Float%20%28single-precision%29) (DamageType :type Damage%20Type%20Object%20Reference) (InstigatedBy :type Controller%20Object%20Reference) (DamageCauser :type Actor%20Object%20Reference))
  (Utilities|FlowControl|DoOnce false
    (:Completed
      (CameraFades|StartCameraFade (Game|GetPlayerCameraManager 0) 1.0 0.0 3.0 "(R=0.108333,G=0.000000,B=0.000648,A=1.000000)" false true)
      (Utilities|FlowControl|Delay 1.0)
      (Game|OpenLevel(byName) "Level01"))))

(event EventBeginPlay
  (CameraFades|StartCameraFade :self (Game|GetPlayerCameraManager 0) :FromAlpha 1.0 :Duration 5.0 :bHoldWhenFinished true))

(event Input|AxisEvents|InputAxismoveforwardback
  (params (AxisValue :type Float%20%28single-precision%29))
  (Class|PrimitiveComponent|AddTorqueinRadians (Variables|Default|GetBP_Ball_01) (Math|Vector|MakeVector 0.0 (* AxisValue 25.0) 0.0) "None" true))

(event Input|AxisEvents|InputAxismoveleftright
  (params (AxisValue :type Float%20%28single-precision%29))
  (Class|PrimitiveComponent|AddTorqueinRadians (Variables|Default|GetBP_Ball_01) (Math|Vector|MakeVector (* AxisValue 25.0) 0.0 0.0) "None" true))

(fn ConstructionScript)